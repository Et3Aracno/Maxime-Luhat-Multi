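; Hit-activated switch that opens doors and starts an on-screen timer, apparently for the lobby going by its name.
; A hit on the Box component swaps the Cube's material and calls DoorOpenMessage on each element of the OpenDoor array.
; TimerStart is called inside that loop, but the BoolTimer flag gates it, clearing once the timer widget is added to the viewport so repeat calls add no duplicates.
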(event OnComponentHit(Box)
  (params (HitComponent :type Primitive%20Component%20Object%20Reference) (OtherActor :type Actor%20Object%20Reference) (OtherComp :type Primitive%20Component%20Object%20Reference) (NormalImpulse :type Vector :default "0, 0, 0") (Hit :type Hit%20Result%20Structure%20%28by%20ref%29))
  ;[0.15 0.15 0.15 0.5] Swap Material / Start Door Custom event
  (Rendering|Material|SetMaterial (Variables|Default|GetCube) 0 "/Game/Assets/MPMECH/MATERIALS/INSTANCES/MAT_MPMECH_01_INST_05.MAT_MPMECH_01_INST_05")
  (for _array_element (Variables|Default|GetOpenDoor)
    (Class|BPIDOOR|DoorOpen(Message) _array_element)
    (CallFunction|TimerStart)))

(event Custom|TimerStart
  ;[0.15 0.15 0.15 0.5] Start Timer
  (if (Variables|Default|GetBoolTimer)
    (bind _returnvalue (UserInterface|CreateWidget "/Game/Widjet/Timer/BP_TIMER_WIDGET.BP_TIMER_WIDGET_C"))
    (UserInterface|Viewport|AddtoViewport _returnvalue 0)
    (Variables|Default|SetBoolTimer false)))

(event EventBeginPlay)

(event Collision|EventActorBeginOverlap
  (params (OtherActor :type Actor%20Object%20Reference)))

(event EventTick
  (params (DeltaSeconds :type Float%20%28single-precision%29)))

(fn ConstructionScript)
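; Double door for the second trial in Level 1, with separate events to open it for Player 1 and Player 2.
; Each event plays its own timeline, whose two rotation tracks are scaled by a shared angle to set the relative yaw of the two door meshes.
; Both events drive the same pair of meshes, and nothing in this Blueprint triggers or closes the door.
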(event EventBeginPlay)

(event Collision|EventActorBeginOverlap
  (params (OtherActor :type Actor%20Object%20Reference)))

(event EventDoorOpenPlayer1
  (bind _rotation_angle_2 (Variables|Default|GetRotation%20Angle%202))
  ;[0.15 0.15 0.15 0.5] Open Player 1 door in second trial
  (bind (_direction _rotation _rottion_02) (Timeline|Timeline Play)
    (:Update
      (Transformation|SetRelativeRotation (Variables|Default|GetSM_Door_01_B) (Math|Rotator|MakeRotator 0.0 0.0 (* _rotation _rotation_angle_2)) false false)
      (Transformation|SetRelativeRotation (Variables|Default|GetSM_Door_01_B1) (Math|Rotator|MakeRotator 0.0 0.0 (* _rottion_02 _rotation_angle_2)) false false))))

(event EventDoorOpenPlayer2
  (bind _rotation_angle_2 (Variables|Default|GetRotation%20Angle%202))
  ;[0.15 0.15 0.15 0.5] Open Player 2 Door in second trial
  (bind (_direction _rotation _rottion_02) (Timeline|Timeline_0 Play)
    (:Update
      (Transformation|SetRelativeRotation (Variables|Default|GetSM_Door_01_B) (Math|Rotator|MakeRotator 0.0 0.0 (* _rotation _rotation_angle_2)) false false)
      (Transformation|SetRelativeRotation (Variables|Default|GetSM_Door_01_B1) (Math|Rotator|MakeRotator 0.0 0.0 (* _rottion_02 _rotation_angle_2)) false false))))

(fn ConstructionScript)
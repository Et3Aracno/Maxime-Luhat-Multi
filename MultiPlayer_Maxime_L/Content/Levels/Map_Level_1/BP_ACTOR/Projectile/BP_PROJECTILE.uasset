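; Projectile actor that spawns a rocket explosion Niagara effect at its mesh when it hits something or runs out of life.
; Its capsule ignores the owner and instigator, and only the authority triggers the explosion and destroys the actor on a hit.
; Lifespan sets the actor's lifespan in seconds, but Tick also decrements it once per frame and explodes when it equals exactly zero.
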(event OnComponentHit(Capsule)
  (params (HitComponent :type Primitive%20Component%20Object%20Reference) (OtherActor :type Actor%20Object%20Reference) (OtherComp :type Primitive%20Component%20Object%20Reference) (NormalImpulse :type Vector :default "0, 0, 0") (Hit :type Hit%20Result%20Structure%20%28by%20ref%29))
  (Networking|SwitchHasAuthority
    (:Authority
      (CallFunction|Explosion)
      (Actor|DestroyActor))))

(event Custom|Explosion
  (bind _staticmesh (Variables|Default|GetStaticMesh))
  (Niagara|SpawnSystematLocation "/Game/Levels/Map_Level_1/BP_ACTOR/Projectile/Rocket_Explosion.Rocket_Explosion" (Transformation|GetWorldLocation _staticmesh) (Transformation|GetWorldRotation _staticmesh)))

(event EventBeginPlay
  (bind _capsule (Variables|Default|GetCapsule))
  (Collision|IgnoreActorwhenMoving _capsule (Components|GetOwner) true)
  (Collision|IgnoreActorwhenMoving _capsule (Game|GetInstigator) true)
  (Actor|SetLifeSpan (Variables|Default|Get%20Lifespan)))

(event Collision|EventActorBeginOverlap
  (params (OtherActor :type Actor%20Object%20Reference)))

(event EventTick
  (params (DeltaSeconds :type Float%20%28single-precision%29))
  (bind _output_get (Variables|Default|Set%20Lifespan (- (Variables|Default|Get%20Lifespan) 1.0)))
  (if (== _output_get 0.0)
    (CallFunction|Explosion)))

(fn ConstructionScript)